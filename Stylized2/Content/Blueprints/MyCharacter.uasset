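; Player character for a soccer game that can take possession of the ball and kick it away.
; Overlapping an unpossessed SoccerBall makes the character its possessor, unless this character kicked it within a brief cooldown window.
; The PrimaryAction input launches the GameMode's ball along the actor's forward vector if this character holds it, recording the time that drives the re-pickup cooldown.
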(event `InputAction|PrimaryAction`
  (:`Pressed`
    ;[1 1 1] If we possess the ball and did a primary action, kick it away
    (bind _asmygamemode_c (cast `/Game/Blueprints/MyGameMode` (`GameplayStatics.GetGameMode`)))
    (bind _soccerball (`/Game/Blueprints/MyGameMode.SoccerBall` _asmygamemode_c))
    (if (== (`/Game/Soccer/Blueprints/SoccerBall.Possessor` _soccerball) self)
      (set `self.LastBallPossessionTime` (`KismetSystemLibrary.GetGameTimeInSeconds`))
      (`/Game/Soccer/Blueprints/SoccerBall.Kick` _soccerball (* (`self.GetActorForwardVector`) 90000.0)))))

(event `self.ReceiveActorBeginOverlap`
  (params (OtherActor :type "Actor Object Reference"))
  ;[1 1 1] See if we overlapped a ball; if so, take possession if nobody else has it and we didn't just possess it 0.2 seconds ago.
  (bind _assoccerball_c (cast `/Game/Soccer/Blueprints/SoccerBall` OtherActor))
  (`/Engine/EditorBlueprintResources/StandardMacros.IsValid` (`/Game/Soccer/Blueprints/SoccerBall.Possessor` _assoccerball_c)
    (:`Is Not Valid`
      (if (> (- (`KismetSystemLibrary.GetGameTimeInSeconds`) (`self.LastBallPossessionTime`)) 0.2)
        (`/Game/Soccer/Blueprints/SoccerBall.SetPossessingPawn` _assoccerball_c self)))))

(fn `UserConstructionScript`
  (`parent.UserConstructionScript`))