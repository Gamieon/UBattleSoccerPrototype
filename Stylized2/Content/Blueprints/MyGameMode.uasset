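; Soccer game mode that sets up the match and acts as the query hub for ball and player information.
; On BeginPlay it caches bots and the ball, teleports them to default field positions, and puts all human players on team 1 by assigning Team2Goal as their enemy goal.
; Helper functions return ball location, possessor, closest actor, and teammates or opponents, inferring team membership by comparing each player's EnemyGoal.
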(event EventBeginPlay
  (CallFunction|CacheSoccerActors)
  ;[1 1 1] Teleport all actors to the field
  (for _array_element (Variables|Default|GetBotTeammates)
    (Default|TeleporttoDefaultFieldPosition _array_element)
    (Default|TeleporttoDefaultFieldPosition (Variables|Default|GetSoccerBall))
    ;[1 1 1] Find the team 2 goal and assign it to the Team2Goal variable
    (bind _outactors (Actor|GetAllActorsOfClass "/Game/Soccer/Goal.Goal_C"))
    (bind _array_element_2 (Utilities|Array|ForEachLoopwithBreak _outactors :!label _label)
      (:LoopBody
        (bind _asgoal_c (Utilities|Casting|CastToGoal _array_element_2))
        (if (Utilities|Enum|Equal(Enum) "Team2Goal" (Utilities|GetDisplayName _asgoal_c))
          (Variables|Default|SetTeam2Goal _asgoal_c)
          (goto _label Break)))
      (:Completed
        ;[1 1 1] Assign every human player the team 2 goal as the enemy goal, thereby assigning every human player to team 1
        (bind _outactors_2 (Actor|GetAllActorsOfClass "/Game/Blueprints/MyCharacter.MyCharacter_C"))
        (for _array_element_3 _outactors_2
          (bind _asmycharacter_c (Utilities|Casting|CastToMyCharacter _array_element_3))
          (Variables|/Game/Blueprints/MyCharacter.MyCharacter_C|SetEnemyGoal _asmycharacter_c (Variables|Default|GetTeam2Goal)))))))

(fn ConstructionScript)

(fn CacheSoccerActors
  (Utilities|Array|Clear (Variables|Default|GetBotTeammates))
  ;[1 1 1] Cache the bot teammates (Both friends and enemies)
  (bind _outactors (Actor|GetAllActorsOfClass "/Game/Soccer/BotTeammate.BotTeammate_C"))
  (for _array_element _outactors
    (bind _asbotteammate_c (Utilities|Casting|CastToBotTeammate _array_element))
    (Utilities|Array|Add (Variables|Default|GetBotTeammates) _asbotteammate_c)
    (Variables|/Game/Soccer/BotTeammate.BotTeammate_C|SetDefaultRotation _asbotteammate_c (Transformation|GetActorRotation _asbotteammate_c)))
  ;[1 1 1] Cache the Soccer Ball
  (bind _outactors_2 (Actor|GetAllActorsOfClass "/Game/Soccer/SoccerBall.SoccerBall_C"))
  (bind _assoccerball_c (Utilities|Casting|CastToSoccerBall (Utilities|Array|Get(acopy) _outactors_2)))
  (Variables|Default|SetSoccerBall _assoccerball_c))

(fn GetBallLocation
  (return (Transformation|GetActorLocation (Variables|Default|GetSoccerBall))))

(fn GetBallPossessor
  (return (Variables|/Game/Soccer/SoccerBall.SoccerBall_C|GetPossessor (Variables|Default|GetSoccerBall))))

(fn GetTeammateActors
  (params (SoccerPlayer :type Actor%20Object%20Reference))
  (LocalVariables|SetSoccerPlayerRef SoccerPlayer)
  (bind _asbotteammate_c (Utilities|Casting|CastToBotTeammate SoccerPlayer)
    (:then
      (LocalVariables|SetSoccerPlayerEnemyGoal (Variables|/Game/Soccer/BotTeammate.BotTeammate_C|GetEnemyGoal _asbotteammate_c)))
    (:CastFailed
      (bind _asmycharacter_c (Utilities|Casting|CastToMyCharacter SoccerPlayer)
        (:then
          (LocalVariables|SetSoccerPlayerEnemyGoal (Variables|/Game/Blueprints/MyCharacter.MyCharacter_C|GetEnemyGoal _asmycharacter_c)))
        (:CastFailed
          _))))
  ;[1 1 1] Find bot teammates
  (for _array_element (Variables|Default|GetBotTeammates)
    (if (== (LocalVariables|GetSoccerPlayerEnemyGoal) (Variables|/Game/Soccer/BotTeammate.BotTeammate_C|GetEnemyGoal _array_element))
      (if (!= _array_element (LocalVariables|GetSoccerPlayerRef))
        (Utilities|Array|Add (LocalVariables|GetFoundTeammates) _array_element))))
  ;[1 1 1] Find player teammates
  (bind _outactors (Actor|GetAllActorsOfClass "/Game/Blueprints/MyCharacter.MyCharacter_C"))
  (for _array_element_2 _outactors
    (bind _asmycharacter_c_2 (Utilities|Casting|CastToMyCharacter _array_element_2))
    (if (== (LocalVariables|GetSoccerPlayerEnemyGoal) (Variables|/Game/Blueprints/MyCharacter.MyCharacter_C|GetEnemyGoal _asmycharacter_c_2))
      (if (!= _asmycharacter_c_2 (LocalVariables|GetSoccerPlayerRef))
        (Utilities|Array|Add (LocalVariables|GetFoundTeammates) _asmycharacter_c_2))))
  (return (LocalVariables|GetFoundTeammates)))

(fn GetClosestActor
  (params (Focus :type Actor%20Object%20Reference) (Actors :type Array%20of%20Actor%20Object%20References))
  ;[1 1 1] Go through the array searching for the actor closest to the "Focus" actor
  (for (_array_element _array_index) Actors
    (bind _returnvalue (Transformation|GetDistanceTo _array_element Focus))
    (if (== _array_index 0)
      (LocalVariables|SetClosestDist _returnvalue :!label _label)
      (LocalVariables|SetClosestDistActor _array_element)
      (elif (< _returnvalue (LocalVariables|GetClosestDist))
        (goto _label))))
  (return (LocalVariables|GetClosestDistActor)))

(fn GetEnemyActors
  (params (SoccerPlayer :type Actor%20Object%20Reference))
  (LocalVariables|SetSoccerPlayerRef SoccerPlayer)
  (bind _asbotteammate_c (Utilities|Casting|CastToBotTeammate SoccerPlayer)
    (:then
      (LocalVariables|SetSoccerPlayerEnemyGoal (Variables|/Game/Soccer/BotTeammate.BotTeammate_C|GetEnemyGoal _asbotteammate_c)))
    (:CastFailed
      (bind _asmycharacter_c (Utilities|Casting|CastToMyCharacter SoccerPlayer)
        (:then
          (LocalVariables|SetSoccerPlayerEnemyGoal (Variables|/Game/Blueprints/MyCharacter.MyCharacter_C|GetEnemyGoal _asmycharacter_c)))
        (:CastFailed
          _))))
  ;[1 1 1] Find bot teammates
  (for _array_element (Variables|Default|GetBotTeammates)
    (if (!= (LocalVariables|GetSoccerPlayerEnemyGoal) (Variables|/Game/Soccer/BotTeammate.BotTeammate_C|GetEnemyGoal _array_element))
      (if (!= _array_element (LocalVariables|GetSoccerPlayerRef))
        (Utilities|Array|Add (LocalVariables|GetFoundTeammates) _array_element))))
  ;[1 1 1] Find player teammates
  (bind _outactors (Actor|GetAllActorsOfClass "/Game/Blueprints/MyCharacter.MyCharacter_C"))
  (for _array_element_2 _outactors
    (bind _asmycharacter_c_2 (Utilities|Casting|CastToMyCharacter _array_element_2))
    (if (!= (LocalVariables|GetSoccerPlayerEnemyGoal) (Variables|/Game/Blueprints/MyCharacter.MyCharacter_C|GetEnemyGoal _asmycharacter_c_2))
      (if (!= _asmycharacter_c_2 (LocalVariables|GetSoccerPlayerRef))
        (Utilities|Array|Add (LocalVariables|GetFoundTeammates) _asmycharacter_c_2))))
  (return (LocalVariables|GetFoundTeammates)))