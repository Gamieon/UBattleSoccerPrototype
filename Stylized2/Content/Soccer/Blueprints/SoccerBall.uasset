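; Soccer ball actor that a pawn can possess, dribble and kick, and that can teleport back to a default field position.
; Possession disables physics simulation and collision, and Tick then holds the ball ahead of the possessor.
; Accumulated pawn speed drives the ball's pitch to fake rolling while it is carried.
; Kick clears possession, restoring physics, then applies the given force; possession changes and overlaps print debug strings.
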(event EventActorBeginOverlap
  (params (OtherActor :type Actor%20Object%20Reference))
  (Development|PrintString (Utilities|String|BuildString(Object) "" "Ball: Begin Overlap (" OtherActor ")") true true "(R=1.000000,G=0.028639,B=0.000000,A=1.000000)"))

(event EventActorEndOverlap
  (params (OtherActor :type Actor%20Object%20Reference))
  (Development|PrintString (Utilities|String|BuildString(Object) "" "Ball: EndOverlap (" OtherActor ")") true true "(R=1.000000,G=0.049789,B=0.068889,A=1.000000)"))

(event EventTick
  (params (DeltaSeconds :type Float%20%28single-precision%29))
  (Utilities|IsValid (Variables|Soccer|GetPossessor)
    (:Is%20Valid
      (CallFunction|MovewithPossessingPawn))))

(fn ConstructionScript)

(fn TeleporttoDefaultFieldPosition
  (Transformation|Teleport (Transformation|GetActorLocation (Variables|Soccer|GetDefaultFieldPositionActor)) "0, 0, 0"))

(fn SetPossessingPawn
  (params (NewPawn :type Pawn%20Object%20Reference))
  ;[1 1 1] Debug Logging
  (Development|PrintString (Utilities|String|BuildString(Object) "" "Ball taken by " NewPawn))
  (Variables|Soccer|SetPossessor NewPawn)
  (Utilities|IsValid NewPawn
    (:Is%20Valid
      (LocalVariables|SetIsNewPawnValid true))
    (:Is%20Not%20Valid
      (LocalVariables|SetIsNewPawnValid false)))
  (bind _asprimitivecomponent (Utilities|Casting|CastToPrimitiveComponent (Utilities|Array|Get(acopy) (Actor|GetComponentsByClass "/Script/Engine.PrimitiveComponent"))))
  (Physics|SetSimulatePhysics _asprimitivecomponent (not (LocalVariables|GetIsNewPawnValid)))
  (Collision|SetActorEnableCollision (not (LocalVariables|GetIsNewPawnValid))))

(fn MovewithPossessingPawn
  (bind _possessor (Variables|Soccer|GetPossessor))
  (Variables|Default|SetNegDistanceTravelled (+ (* (Math|Vector|VectorLength (Transformation|GetVelocity _possessor)) -0.01) (Variables|Default|GetNegDistanceTravelled)))
  (Transformation|SetActorLocation (+ (Transformation|GetActorLocation _possessor) (* (Transformation|GetActorForwardVector _possessor) 9e+01) "0,0,-60.000000") false)
  (Transformation|SetActorRotation (Class|KismetMathLibrary|MakeRot (+ (* (Math|Vector|VectorLength (Transformation|GetVelocity _possessor)) -0.01) (Variables|Default|GetNegDistanceTravelled)) (.Yaw (Class|KismetMathLibrary|BreakRot (Transformation|GetActorRotation _possessor))) 0.0)))

(fn Kick
  (params (Force :type Vector))
  (CallFunction|SetPossessingPawn)
  (bind _asprimitivecomponent (Utilities|Casting|CastToPrimitiveComponent (Utilities|Array|Get(acopy) (Actor|GetComponentsByClass "/Script/Engine.PrimitiveComponent"))))
  (Physics|AddForce _asprimitivecomponent Force "None"))