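; Destructible enemy spawner that periodically spawns Enemy actors with default controllers at its SpawnPoint.
; Fireballs overlapping DamageBox are destroyed and remove one hitpoint, destroying the spawner at zero.
; Remaining hitpoints map to a rounded-up tier whose fraction of Maxtier scales both spawn interval and actor size.
; Each surviving hit restarts the looping timer, so a more damaged spawner shrinks and spawns faster as tiers drop.
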(event `self.ReceiveBeginPlay`
  (set `self.hitpoints` (`self.maxhitpoints`))
  (set `self.initialscale` (`self.GetActorScale3D`))
  (bind _interval (`self.GetSpawnInterval`))
  (`KismetSystemLibrary.K2_SetTimer` null "SpawnEnemy" _interval true))

(event `self.DamageBox.OnComponentBeginOverlap`
  (params (OtherActor :type "Actor Object Reference") (OtherComp :type "PrimitiveComponent Object Reference") (OtherBodyIndex :type Integer) (bFromSweep :type Boolean) (SweepResult :type "EngineTypes.HitResult Structure (by ref)"))
  (bind _asfireball_c (cast `/Game/Blueprints/Fireball` OtherActor))
  (`self.K2_DestroyActor` _asfireball_c)
  (set `self.hitpoints` (- (`self.hitpoints`) 1))
  (if (== (`self.hitpoints`) 0)
    (`self.K2_DestroyActor`)
    (else
      (`KismetSystemLibrary.K2_ClearTimer` null "SpawnEnemy")
      (bind _interval (`self.GetSpawnInterval`))
      (`KismetSystemLibrary.K2_SetTimer` null "SpawnEnemy" _interval true)
      (bind _scale (`self.GetAdjustedScale` (`self.initialscale`)))
      (`self.SetActorScale3D` _scale))))

(fn `GetAdjustedScale`
  (params (InitialScale :type "Object.Vector Structure"))
  (returns (Scale :type "Object.Vector Structure"))
  (bind _currenttier (`self.GetCurrentTier`))
  (return (* InitialScale (/ (`KismetMathLibrary.Conv_IntToDouble` _currenttier) (`KismetMathLibrary.Conv_IntToDouble` (`self.maxtier`))))))

(fn `GetCurrentTier`
  (returns (CurrentTier :type Integer))
  (return (`KismetMathLibrary.FCeil` (/ (`KismetMathLibrary.Conv_IntToDouble` (* (`self.hitpoints`) (`self.maxtier`))) (`KismetMathLibrary.Conv_IntToDouble` (`self.maxhitpoints`))))))

(fn `GetSpawnInterval`
  (returns (Interval :type "Float (double-precision)"))
  (bind _currenttier (`self.GetCurrentTier`))
  (return (* (/ (`KismetMathLibrary.Conv_IntToDouble` _currenttier) (`KismetMathLibrary.Conv_IntToDouble` (`self.maxtier`))) 4.0)))

(fn `SpawnEnemy`
  (bind _returnvalue (`|SpawnActorFromClass` "/Game/Blueprints/Enemy.Enemy_C" (`SceneComponent.K2_GetComponentToWorld` (`self.SpawnPoint`)) true))
  (`Pawn.SpawnDefaultController` _returnvalue))

(fn `UserConstructionScript`)