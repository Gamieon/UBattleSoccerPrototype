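; Soccer player Blueprint that shows a stun indicator and sets the player's team uniform.
; Each tick, Star1's visibility follows IsStunned while the star spins around its yaw axis at a frame-rate-independent speed.
; AssignUniform checks the EnemyGoal display name and, for Team1Goal, swaps in the red Exo skeletal mesh and its matching animation Blueprint.
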(event `self.ReceiveBeginPlay`
  ;[1 1 1] Event Begin Play
  (`SceneComponent.SetVisibility` (`self.Star1`) false false))

(event `self.ReceiveTick`
  (params (DeltaSeconds :type "Float (single-precision)"))
  (bind _star1 (`self.Star1`))
  ;[1 1 1] Event Tick
  (`SceneComponent.SetVisibility` _star1 (`self.IsStunned`) false)
  (`SceneComponent.AddRelativeRotation` _star1 (`KismetMathLibrary.MakeRot` 0.0 (* DeltaSeconds 200.0)) false))

(fn `AssignUniform`
  (if (`KismetStringLibrary.EqualEqual_StrStr` (`KismetSystemLibrary.GetDisplayName` (`self.EnemyGoal`)) "Team1Goal")
    (bind _asskinnedmeshcomponent (cast `SkinnedMeshComponent` (`KismetArrayLibrary.Array_Get` (`self.K2_GetComponentsByClass` "/Script/Engine.SkinnedMeshComponent"))))
    (`SkinnedMeshComponent.SetSkinnedAssetAndUpdate` _asskinnedmeshcomponent "/Game/MixamoAnimPack/Mixamo_ExoRed/Mesh/Maximo_ExoRed.Maximo_ExoRed")
    (bind _asskeletalmeshcomponent (cast `SkeletalMeshComponent` (`KismetArrayLibrary.Array_Get` (`self.K2_GetComponentsByClass` "/Script/Engine.SkeletalMeshComponent"))))
    (`SkeletalMeshComponent.SetAnimInstanceClass` _asskeletalmeshcomponent "/Game/MixamoAnimPack/Mixamo_ExoRed/Anims/MixamoAnimBP_ExoRed.MixamoAnimBP_ExoRed_C")))

(fn `UserConstructionScript`)