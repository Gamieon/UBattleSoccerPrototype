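; Soccer player controller that lets a player respawn through the Respawn input when no pawn is controlled.
; On authority, such as a listen-server host, it calls Respawn on SoccerGameMode directly, passing itself.
; Remote clients call RequestRespawn, which checks for authority before making the same game mode call.
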(event `InputAction|Respawn`
  (:`Pressed`
    (`/Engine/EditorBlueprintResources/StandardMacros.IsValid` (`self.K2_GetPawn`)
      (:`Is Not Valid`
        (`/Engine/EditorBlueprintResources/ActorMacros.Switch Has Authority`
          (:`Authority`
            ;[1 1 1] Non-dedicated server player respawning
            (bind _assoccergamemode_c (cast `/Game/Soccer/Blueprints/SoccerGameMode` (`GameplayStatics.GetGameMode`)))
            (bind _returnvalue (`self.CastToPlayerController` self))
            (`/Game/Soccer/Blueprints/SoccerGameMode.Respawn` _assoccergamemode_c _returnvalue))
          (:`Remote`
            ;[1 1 1] Client respawning
            (`self.RequestRespawn`)))))))

(event `RequestRespawn`
  (`/Engine/EditorBlueprintResources/ActorMacros.Switch Has Authority`
    (:`Authority`
      (bind _assoccergamemode_c (cast `/Game/Soccer/Blueprints/SoccerGameMode` (`GameplayStatics.GetGameMode`)))
      (bind _returnvalue (`self.CastToPlayerController` self))
      (`/Game/Soccer/Blueprints/SoccerGameMode.Respawn` _assoccergamemode_c _returnvalue))))

(fn `UserConstructionScript`)