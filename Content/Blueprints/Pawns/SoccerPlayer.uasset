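; SoccerPlayer is the player pawn Blueprint for Magic Battle Soccer, handling the team uniform.
; The AssignUniform event calls ChangeSkin, which reads the team number from the MagicBattleSoccerPlayerState.
; For team 2 it swaps the first skinned mesh component to the red Exo mesh and sets the matching animation Blueprint.
; Other teams keep their default look, and the construction script is empty.
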(event `self.AssignUniform`
  (`self.ChangeSkin`))

(fn `ChangeSkin`
  (bind _asmagicbattlesoccerplayerstate (cast `MagicBattleSoccerPlayerState` (`self.PlayerState`)))
  (if (== (`MagicBattleSoccerPlayerState.TeamNumber` _asmagicbattlesoccerplayerstate) 2)
    (bind _asskinnedmeshcomponent (cast `SkinnedMeshComponent` (`KismetArrayLibrary.Array_Get` (`self.K2_GetComponentsByClass` "/Script/Engine.SkinnedMeshComponent"))))
    (`SkinnedMeshComponent.SetSkinnedAssetAndUpdate` _asskinnedmeshcomponent "/Game/MixamoAnimPack/Mixamo_ExoRed/Mesh/Maximo_ExoRed.Maximo_ExoRed")
    (bind _asskeletalmeshcomponent (cast `SkeletalMeshComponent` (`KismetArrayLibrary.Array_Get` (`self.K2_GetComponentsByClass` "/Script/Engine.SkeletalMeshComponent"))))
    (`SkeletalMeshComponent.SetAnimInstanceClass` _asskeletalmeshcomponent "/Game/MixamoAnimPack/Mixamo_ExoRed/Anims/MixamoAnimBP_ExoRed.MixamoAnimBP_ExoRed_C")))

(fn `UserConstructionScript`)