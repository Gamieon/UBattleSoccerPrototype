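; Player controller that spawns and possesses the human player's soccer character for their team.
; SpawnCharacter runs only with authority and proceeds when CanSpawnCharacter allows it.
; It reads the team number from the player state, then scans all SoccerSpawnPoint actors for matching team points flagged for human players.
; At each match it spawns a SoccerPlayer, even if colliding, and possesses it; the loop has no early exit.
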(event `self.SpawnCharacter`
  (`/Engine/EditorBlueprintResources/ActorMacros.Switch Has Authority`
    (:`Authority`
      (`self.CanSpawnCharacter`)
      (if true
        (bind _asmagicbattlesoccerplayerstate (cast `MagicBattleSoccerPlayerState` (`self.PlayerState`)))
        ;[1 1 1] Find the spawn point for our team that spawns human players
        (bind _outactors (`GameplayStatics.GetAllActorsOfClass` "/Game/Blueprints/Soccer/SoccerSpawnPoint.SoccerSpawnPoint_C"))
        (for _array_element _outactors
          (bind _assoccerspawnpoint_c (cast `/Game/Blueprints/Soccer/SoccerSpawnPoint` _array_element))
          (if (== (`MagicBattleSoccerSpawnPoint.OwningTeamNumber` _assoccerspawnpoint_c) (`MagicBattleSoccerPlayerState.TeamNumber` _asmagicbattlesoccerplayerstate))
            (if (`MagicBattleSoccerSpawnPoint.SpawnHumanPlayers` _assoccerspawnpoint_c)
              ;[1 1 1] Spawn the human player
              (bind _returnvalue (`|SpawnActorFromClass` "/Game/Blueprints/Pawns/SoccerPlayer.SoccerPlayer_C" (`self.GetTransform` _assoccerspawnpoint_c) true))
              (`self.Possess` _returnvalue))))))))

(fn `UserConstructionScript`)