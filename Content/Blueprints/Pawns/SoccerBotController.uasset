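; AI controller for soccer bots in a Magic Battle Soccer game, responsible for spawning and driving their characters.
; On the server, when spawning is allowed, it picks a class by team (team 1 gets Noah, others randomly Guard or Noah), spawns it at a spawn point, possesses it and runs BT_Bot.
; Round start and end call the parent handlers, then clear any pending spawn timer.
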(event EventSpawnCharacter
  (CallFunction|SpawnCharacterInternal))

(event EventRoundHasEnded
  (|CallParentFunction)
  (Utilities|Time|ClearTimerbyFunctionName 0 "SpawnCharacterInternal"))

(event EventRoundHasStarted
  (|CallParentFunction)
  (Utilities|Time|ClearTimerbyFunctionName 0 "SpawnCharacterInternal"))

(fn ConstructionScript)

(fn SpawnCharacterInternal
  (Networking|SwitchHasAuthority
    (:Authority
      (bind _returnvalue (Class|MagicBattleSoccerAIController|CanSpawnCharacter))
      (if _returnvalue
        (bind _asmagic_battle_soccer_player_state (Utilities|Casting|CastToMagicBattleSoccerPlayerState (Variables|Default|GetPlayerState)))
        (if (== (Variables|/Script/MagicBattleSoccer.MagicBattleSoccerPlayerState|GetTeamNumber _asmagic_battle_soccer_player_state) 1)
          (LocalVariables|SetClassToSpawn "/Game/Characters/Noah/noah.Noah_C")
          (elif (Math|Random|RandomBool)
            (LocalVariables|SetClassToSpawn "/Game/Characters/Guard/Guard.Guard_C")
            (else
              (LocalVariables|SetClassToSpawn "/Game/Characters/Noah/noah.Noah_C"))))
        (bind _returnvalue_2 (Game|SpawnActorfromClass (LocalVariables|GetClassToSpawn) (Transformation|GetActorTransform (Variables|Default|GetSpawnPoint)) true 0))
        (Pawn|Possess _returnvalue_2)
        (AI|RunBehaviorTree "/Game/Blueprints/AI/BT_Bot.BT_Bot")))))