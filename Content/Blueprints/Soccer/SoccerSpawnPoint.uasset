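; Spawn point for Magic Battle Soccer that, on the server, keeps its number of AI soccer players on the field up to a maximum.
; At BeginPlay it counts pre-placed players already assigned to it, then spawns the rest.
; Each new player gets an AI controller with the enemy goal and action zone, a link back to the spawn point, and a uniform.
; When notified that a player is being destroyed, it schedules a delayed respawn.
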(event `self.ReceiveBeginPlay`
  (`/Engine/EditorBlueprintResources/ActorMacros.Switch Has Authority`
    (:`Authority`
      ;[1 1 1] Find existing players that already have us as a spawn point (should only be in test scenes) and increment the existing spawned player count
      (bind _outactors (`GameplayStatics.GetAllActorsOfClass` "/Script/MagicBattleSoccer.MagicBattleSoccerPlayer"))
      (for _array_element _outactors
        (bind _asmagicbattlesoccerplayer (cast `MagicBattleSoccerPlayer` _array_element))
        (if (== self (`MagicBattleSoccerPlayer.SpawnPoint` _asmagicbattlesoccerplayer))
          (set `self.NumberOfPlayersOnField` (+ (`self.NumberOfPlayersOnField`) 1))))
      ;[1 1 1] Spawn soccer players until we reach our limit
      (while (< (`self.NumberOfPlayersOnField`) (`self.MaxPlayersOnField`))
        (`self.SpawnSoccerPlayer`)))))

(event `self.SpawnedPlayerBeingDestroyed`
  (params (SoccerPlayer :type "MagicBattleSoccerPlayer Object Reference"))
  (`/Engine/EditorBlueprintResources/ActorMacros.Switch Has Authority`
    (:`Authority`
      (set `self.NumberOfPlayersOnField` (- (`self.NumberOfPlayersOnField`) 1))
      (`KismetSystemLibrary.K2_SetTimer` null "SpawnSoccerPlayer" 3.0))))

(fn `SpawnSoccerPlayer`
  (bind _returnvalue (`|SpawnActorFromClass` "/Game/Blueprints/Pawns/SoccerPlayer.SoccerPlayer_C" (`self.GetTransform`) true))
  (`Pawn.SpawnDefaultController` _returnvalue)
  (bind _asmagicbattlesocceraicontroller (cast `MagicBattleSoccerAIController` (`Pawn.GetController` _returnvalue)))
  (set `MagicBattleSoccerAIController.EnemyGoal` (`self.EnemyGoal`) _asmagicbattlesocceraicontroller)
  (set `MagicBattleSoccerAIController.ActionZone` (`self.ActionZone`) _asmagicbattlesocceraicontroller)
  (set `MagicBattleSoccerPlayer.SpawnPoint` self _returnvalue)
  (`/Game/Blueprints/Pawns/SoccerPlayer.AssignUniform` _returnvalue)
  (set `self.NumberOfPlayersOnField` (+ (`self.NumberOfPlayersOnField`) 1)))

(fn `UserConstructionScript`)