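; Behavior tree task for soccer bots that handles the celebration after a goal.
; It stops the controlled character's movement immediately and sets the bot controller's behavior string to Dancing.
; It then finishes at once, succeeding only if the penetrated goal's team number in the game state matches the player's team, as a check on whether the team scored.
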(event `self.ReceiveExecute`
  (params (OwnerActor :type "Actor Object Reference"))
  ;[1 1 1] Get the controlled soccer player
  (bind _assoccer_bot_controller (cast `/Game/Blueprints/Pawns/SoccerBotController` OwnerActor))
  (bind _asmagic_battle_soccer_character (cast `MagicBattleSoccerCharacter` (`Controller.K2_GetPawn` _assoccer_bot_controller)))
  ;[1 1 1] Stop moving immediately
  (`MovementComponent.StopMovementImmediately` (`Pawn.GetMovementComponent` _asmagic_battle_soccer_character))
  ;[1 1 1] Determine if our team scored
  (bind _asmagic_battle_soccer_player_state (cast `MagicBattleSoccerPlayerState` (`Pawn.PlayerState` _asmagic_battle_soccer_character)))
  (bind _asmagic_battle_soccer_game_state (cast `MagicBattleSoccerGameState` (`GameplayStatics.GetGameState`)))
  (set `/Game/Blueprints/Pawns/SoccerBotController.CurrentBehaviorString` "Dancing" _assoccer_bot_controller)
  (`self.FinishExecute` (not (!= (`MagicBattleSoccerGoal.TeamNumber` (`MagicBattleSoccerGameState.PenetratedGoal` _asmagic_battle_soccer_game_state)) (`MagicBattleSoccerPlayerState.TeamNumber` _asmagic_battle_soccer_player_state)))))