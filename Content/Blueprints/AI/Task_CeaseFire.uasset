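; Behavior tree task that makes a Magic Battle Soccer AI stop attacking when it is not pursuing an opponent.
; On execute, if the AI controller is attacking, it calls StopAttackingPlayer when the PursuitActor blackboard value is invalid or is the soccer ball.
; It finishes as failed whether or not it ceases fire, so it never reports success to the tree.
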(event `self.ReceiveExecute`
  (params (OwnerActor :type "Actor Object Reference"))
  (bind _returnvalue (`BTFunctionLibrary.GetBlackboardValueAsObject` (make `BehaviorTreeTypes.BlackboardKeySelector` (`|MakeArray` null :!type "BlackboardKeyType Object Reference") "PursuitActor")))
  ;[1 1 1] Determine if we're attacking an opponent
  (bind _asmagic_battle_soccer_aicontroller (cast `MagicBattleSoccerAIController` OwnerActor))
  (bind _returnvalue_2 (`MagicBattleSoccerAIController.IsAttacking` _asmagic_battle_soccer_aicontroller))
  (if _returnvalue_2
    ;[1 1 1] Are we pursuing an enemy?
    (`/Engine/EditorBlueprintResources/StandardMacros.IsValid` _returnvalue
      (:`Is Valid`
        (cast `/Game/Blueprints/Soccer/SoccerBall` _returnvalue
          (:`then`
            (`MagicBattleSoccerAIController.StopAttackingPlayer` _asmagic_battle_soccer_aicontroller :!label _label))
          (:`CastFailed`
            _)))
      (:`Is Not Valid`
        (goto _label)))
    (`self.FinishExecute` false)
    (else
      (`self.FinishExecute` false))))