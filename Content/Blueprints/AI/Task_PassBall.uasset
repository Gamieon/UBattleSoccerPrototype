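; PassBall is a Behavior Tree task that makes a Magic Battle Soccer AI pass the ball to a teammate.
; It reads the PassToSoccerPlayer blackboard object and has the owning AI controller kick the ball to that character's location.
; A missing target sets KickFailed, which FinishExecute receives directly as its success value on both paths.
; A failed cast stops execution without finishing the task.
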(event `self.ReceiveExecute`
  (params (OwnerActor :type "Actor Object Reference"))
  (bind _returnvalue (`BTFunctionLibrary.GetBlackboardValueAsObject` (make `BehaviorTreeTypes.BlackboardKeySelector` (`|MakeArray` null :!type "BlackboardKeyType Object Reference") "PassToSoccerPlayer")))
  (`/Engine/EditorBlueprintResources/StandardMacros.IsValid` _returnvalue
    (:`Is Valid`
      (bind _asmagicbattlesoccercharacter (cast `MagicBattleSoccerCharacter` _returnvalue))
      (bind _asmagicbattlesocceraicontroller (cast `MagicBattleSoccerAIController` OwnerActor))
      (`MagicBattleSoccerAIController.KickBallToLocation` _asmagicbattlesocceraicontroller (`Actor.K2_GetActorLocation` _asmagicbattlesoccercharacter)))
    (:`Is Not Valid`
      (set `self.KickFailed` true)))
  (`self.FinishExecute` (`self.KickFailed`)))