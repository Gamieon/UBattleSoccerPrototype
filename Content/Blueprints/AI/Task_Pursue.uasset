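; Behavior tree task that drives a soccer bot toward the actor in the PursuitActor blackboard key and updates its behavior string.
; Opponents within primary weapon range, or a default range without a weapon, are attacked.
; Other targets get a simple move order to their location clipped to the bot's action zone.
; It never waits for arrival, finishing as failed while a target exists and succeeded when none does.
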(event EventReceiveExecute
  (params (OwnerActor :type Actor%20Object%20Reference))
  (bind _array (Utilities|Array|MakeArray 0))
  (bind _blackboardkeyselector (Utilities|Struct|MakeBlackboardKeySelector _array "PursuitActor"))
  (bind _returnvalue (Class|BTFunctionLibrary|GetBlackboardValueasObject _blackboardkeyselector))
  ;[1 1 1] Cache values for easier reading
  (bind _assoccer_bot_controller (Utilities|Casting|CastToSoccerBotController OwnerActor))
  (Variables|Default|SetMySoccerBotControllerRef _assoccer_bot_controller)
  (bind _asmagic_battle_soccer_character (Utilities|Casting|CastToMagicBattleSoccerCharacter (Pawn|GetControlledPawn _assoccer_bot_controller)))
  (Variables|Default|SetMyCharacterRef _asmagic_battle_soccer_character)
  ;[1 1 1] Determine if we're pursuing anything
  (Utilities|IsValid _returnvalue
    (:Is%20Valid
      (bind _asactor (Utilities|Casting|CastToActor _returnvalue))
      (bind _behaviorstring (CallFunction|GetBehaviorString _asactor))
      (Variables|/Game/Blueprints/Pawns/SoccerBotController.SoccerBotController_C|SetCurrentBehaviorString (Variables|Default|GetMySoccerBotControllerRef) (Utilities|String|Append "Pursuing " _behaviorstring))
      ;[1 1 1] Cache the pursuit actor's location
      (Variables|Default|SetTargetLocation (Transformation|GetActorLocation _asactor))
      (bind _asmagic_battle_soccer_character_2 (Utilities|Casting|CastToMagicBattleSoccerCharacter _asactor)
        (:then
          ;[1 1 1] Is the pursuit actor an opponent?
          (bind _returnvalue_2 (Class|MagicBattleSoccerAIController|GetOpponents (Variables|Default|GetMySoccerBotControllerRef)))
          (if (Utilities|Array|ContainsItem _returnvalue_2 _asmagic_battle_soccer_character_2)
            ;[1 1 1] Determine if the opponent is close
            (Utilities|IsValid (Variables|/Script/MagicBattleSoccer.MagicBattleSoccerCharacter|GetPrimaryWeapon (Variables|Default|GetMyCharacterRef))
              (:Is%20Valid
                (Variables|Default|SetEffectiveRange (.EffectiveRange (Utilities|Struct|BreakWeaponData (Variables|/Script/MagicBattleSoccer.MagicBattleSoccerWeapon|GetWeaponConfig (Variables|/Script/MagicBattleSoccer.MagicBattleSoccerCharacter|GetPrimaryWeapon (Variables|Default|GetMyCharacterRef)))))))
              (:Is%20Not%20Valid
                (Variables|Default|SetEffectiveRange 2e+02)))
            (if (< (Math|Vector|VectorLength (- (Variables|Default|GetTargetLocation) (Transformation|GetActorLocation (Variables|Default|GetMyCharacterRef)))) (Variables|Default|GetEffectiveRange))
              ;[1 1 1] Attack the opponent
              (Class|MagicBattleSoccerAIController|AttackPlayer (Variables|Default|GetMySoccerBotControllerRef) _asmagic_battle_soccer_character_2)
              (else
                ;[1 1 1] Move to the actor
                (bind _returnvalue_3 (Class|MagicBattleSoccerAIController|CliptoActionZone (Variables|Default|GetMySoccerBotControllerRef) (Variables|Default|GetTargetLocation) :!label _label))
                (AI|Navigation|SimpleMovetoLocation (Variables|Default|GetMySoccerBotControllerRef) _returnvalue_3)))
            (else
              (goto _label))))
        (:CastFailed
          (goto _label)))
      (AI|BehaviorTree|FinishExecute false))
    (:Is%20Not%20Valid
      (AI|BehaviorTree|FinishExecute true))))

(fn GetBehaviorString
  (params (Actor :type Actor%20Object%20Reference))
  (bind _asmagic_battle_soccer_character (Utilities|Casting|CastToMagicBattleSoccerCharacter Actor)
    (:then
      (LocalVariables|SetActorName (Variables|/Script/Engine.PlayerState|GetPlayerName (Variables|/Script/Engine.Pawn|GetPlayerState _asmagic_battle_soccer_character))))
    (:CastFailed
      (Utilities|Casting|CastToSoccerBall Actor
        (:then
          (LocalVariables|SetActorName "soccer ball"))
        (:CastFailed
          (LocalVariables|SetActorName "other actor")))))
  (return (LocalVariables|GetActorName)))