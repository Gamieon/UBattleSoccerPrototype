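; Behavior tree task that lets an AI Magic Battle Soccer character choose between its primary and secondary weapon and fire it.
; Each weapon's score sums the health change on affected actors, weighted by their closeness to the ball, and picks the top contributor as target.
; The higher-scoring weapon fires at the target's velocity-adjusted location if above a minimum threshold, while the other stops.
; Non-repeating weapons are stopped before each shot so they can retrigger.
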(event EventReceiveExecute
  (params (OwnerActor :type Actor%20Object%20Reference))
  (bind _asmagic_battle_soccer_aicontroller (Utilities|Casting|CastToMagicBattleSoccerAIController OwnerActor))
  (bind _asmagic_battle_soccer_character (Utilities|Casting|CastToMagicBattleSoccerCharacter (Pawn|GetControlledPawn _asmagic_battle_soccer_aicontroller)))
  (Variables|Default|SetCachedCharacter _asmagic_battle_soccer_character)
  (Variables|Default|SetCachedPrimaryWeapon (Variables|/Script/MagicBattleSoccer.MagicBattleSoccerCharacter|GetPrimaryWeapon _asmagic_battle_soccer_character))
  (Variables|Default|SetCachedSecondaryWeapon (Variables|/Script/MagicBattleSoccer.MagicBattleSoccerCharacter|GetSecondaryWeapon _asmagic_battle_soccer_character))
  ;[1 1 1] Get the effectiveness of each weapon
  (bind (_effectivenessvalue _idealactor) (CallFunction|GetCurrentEffectivenessValue (Variables|/Script/MagicBattleSoccer.MagicBattleSoccerCharacter|GetPrimaryWeapon _asmagic_battle_soccer_character)))
  (bind (_effectivenessvalue_2 _idealactor_2) (CallFunction|GetCurrentEffectivenessValue (Variables|/Script/MagicBattleSoccer.MagicBattleSoccerCharacter|GetSecondaryWeapon _asmagic_battle_soccer_character)))
  ;[1 1 1] Now determine which weapon (if any) to fire based on the effectiveness of the two weapons.
  (if (>= _effectivenessvalue _effectivenessvalue_2)
    ;[1 1 1] Stop firing the weapon we know we're not firing in this frame.
    (Utilities|IsValid (Variables|Default|GetCachedSecondaryWeapon)
      (:Is%20Valid
        (Class|MagicBattleSoccerCharacter|StopWeaponFire (Variables|Default|GetCachedCharacter) (Variables|Default|GetCachedSecondaryWeapon)))
      (:Is%20Not%20Valid
        _))
    ;[1 1 1] Fire the weapon
    (Utilities|IsValid (Variables|Default|GetCachedPrimaryWeapon)
      (:Is%20Valid
        (CallFunction|FireWeapon (Variables|Default|GetCachedPrimaryWeapon) (> _effectivenessvalue (Variables|Default|GetAllowedMinimum)) _idealactor))
      (:Is%20Not%20Valid
        _))
    (else
      (Utilities|IsValid (Variables|Default|GetCachedPrimaryWeapon)
        (:Is%20Valid
          (Class|MagicBattleSoccerCharacter|StopWeaponFire (Variables|Default|GetCachedCharacter) (Variables|Default|GetCachedPrimaryWeapon)))
        (:Is%20Not%20Valid
          _))
      (Utilities|IsValid (Variables|Default|GetCachedSecondaryWeapon)
        (:Is%20Valid
          (CallFunction|FireWeapon (Variables|Default|GetCachedSecondaryWeapon) (> _effectivenessvalue_2 (Variables|Default|GetAllowedMinimum)) _idealactor_2))
        (:Is%20Not%20Valid
          _))))
  (AI|BehaviorTree|FinishExecute true))

(fn IsFiring
  (params (Weapon :type Magic%20Battle%20Soccer%20Weapon%20Object%20Reference))
  (Utilities|IsValid Weapon
    (:Is%20Valid
      (LocalVariables|Set_Firing (Utilities|Enum|Equal(Enum) (Class|MagicBattleSoccerWeapon|GetCurrentState Weapon) "Firing")))
    (:Is%20Not%20Valid
      (LocalVariables|Set_Firing false)))
  (return (LocalVariables|Get_Firing)))

(fn GetCurrentEffectivenessValue
  (params (Weapon :type Magic%20Battle%20Soccer%20Weapon%20Object%20Reference))
  (Utilities|IsValid Weapon
    (:Is%20Valid
      ;[1 1 1] Cache the soccer ball
      (bind _asmagic_battle_soccer_game_state (Utilities|Casting|CastToMagicBattleSoccerGameState (Game|GetGameState)))
      (LocalVariables|SetSoccerBall (Variables|/Script/MagicBattleSoccer.MagicBattleSoccerGameState|GetSoccerBall _asmagic_battle_soccer_game_state))
      (bind _returnvalue (Class|MagicBattleSoccerWeapon|GetCurrentEffectiveness Weapon))
      (for _array_element _returnvalue
        ;[1 1 1] Get the sum of all effectiveness values and store them into "value"
        (bind _returnvalue_2 (Transformation|GetDistanceTo (.Actor (Utilities|Struct|BreakWeaponActorEffectiveness _array_element)) (LocalVariables|GetSoccerBall)))
        (LocalVariables|SetCalculatedEffectiveness (+ (* (.HealthChange (Utilities|Struct|BreakWeaponActorEffectiveness _array_element)) (- 1e+01 (Math|Float|Clamp(Float) (/ _returnvalue_2 1e+03) 0.0 1e+01))) (LocalVariables|GetCalculatedEffectiveness)))
        ;[1 1 1] Determine the ideal target location
        (Utilities|IsValid (LocalVariables|GetIdealTargetActor)
          (:Is%20Valid
            (if (< (LocalVariables|GetIdealTargetValue) (* (.HealthChange (Utilities|Struct|BreakWeaponActorEffectiveness _array_element)) (- 1e+01 (Math|Float|Clamp(Float) (/ _returnvalue_2 1e+03) 0.0 1e+01))))
              (LocalVariables|SetIdealTargetActor (.Actor (Utilities|Struct|BreakWeaponActorEffectiveness _array_element)) :!label _label)
              (LocalVariables|SetIdealTargetValue (* (.HealthChange (Utilities|Struct|BreakWeaponActorEffectiveness _array_element)) (- 1e+01 (Math|Float|Clamp(Float) (/ _returnvalue_2 1e+03) 0.0 1e+01))))))
          (:Is%20Not%20Valid
            (goto _label)))))
    (:Is%20Not%20Valid
      _))
  (return (LocalVariables|GetCalculatedEffectiveness) (LocalVariables|GetIdealTargetActor)))

(fn FireWeapon
  (params (Weapon :type Magic%20Battle%20Soccer%20Weapon%20Object%20Reference) (Fire :type Boolean) (Target :type Actor%20Object%20Reference))
  (LocalVariables|SetCachedWeapon Weapon)
  (LocalVariables|SetCachedTarget Target)
  (if Fire
    ;[1 1 1] If the weapon is not repeating fire, then stop firing first. If we don't do this, it's the equivalent of holding the "fire" button while doing non repeating attacks; meaning they'd only happen once ever.
    (if (.RepeatingFire (Utilities|Struct|BreakWeaponData (Variables|/Script/MagicBattleSoccer.MagicBattleSoccerWeapon|GetWeaponConfig (LocalVariables|GetCachedWeapon))))
      _
      (else
        (Class|MagicBattleSoccerCharacter|StopWeaponFire (Variables|Default|GetCachedCharacter) (LocalVariables|GetCachedWeapon))))
    ;[1 1 1] Set the weapon's target so it knows where to fire
    (bind _aspawn (Utilities|Casting|CastToPawn (LocalVariables|GetCachedTarget)))
    (Class|MagicBattleSoccerWeapon|SetTargetLocationAdjustedforVelocity (LocalVariables|GetCachedWeapon) (Transformation|GetActorLocation (LocalVariables|GetCachedTarget)) (Transformation|GetVelocity _aspawn))
    (Class|MagicBattleSoccerCharacter|StartWeaponFire (Variables|Default|GetCachedCharacter) (LocalVariables|GetCachedWeapon))
    (else
      ;[1 1 1] We're not firing the weapon, so ensure firing has stopped.
      (Class|MagicBattleSoccerCharacter|StopWeaponFire (Variables|Default|GetCachedCharacter) (LocalVariables|GetCachedWeapon)))))