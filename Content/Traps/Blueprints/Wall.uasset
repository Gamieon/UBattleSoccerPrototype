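; Temporary wall trap actor that rises out of the ground, holds briefly, then sinks back and destroys itself.
; BeginPlay records spawn location, precomputes rise-end and fall-start timestamps, sets its lifespan to match, and drops the wall below ground.
; Tick picks the phase from game time and lerps Z between fixed world heights for rising and sinking, snapping to the spawn location while raised.
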(event `self.ReceiveBeginPlay`
  (bind _returnvalue (`self.K2_GetActorLocation`))
  (bind _returnvalue_2 (`KismetSystemLibrary.GetGameTimeInSeconds`))
  (bind _returnvalue_3 (+ _returnvalue_2 (`self.RiseFallDuration`)))
  (bind _returnvalue_4 (+ _returnvalue_3 2.0))
  (set `self.SpawnTime` _returnvalue_2)
  (set `self.RisenTime` _returnvalue_3)
  (set `self.FallTime` _returnvalue_4)
  (`self.SetLifeSpan` (+ _returnvalue_4 (`self.RiseFallDuration`)))
  (set `self.SpawnLocation` _returnvalue)
  (`self.K2_SetActorLocation` (`KismetMathLibrary.MakeVector` (.x _returnvalue) (.y _returnvalue) -300.0)))

(event `self.ReceiveTick`
  (params (DeltaSeconds :type "Float (single-precision)"))
  (if (> (`KismetSystemLibrary.GetGameTimeInSeconds`) (`self.FallTime`))
    ;[1 1 1] Sink the wall
    (`self.K2_SetActorLocation` (`KismetMathLibrary.MakeVector` (.x (`self.SpawnLocation`)) (.y (`self.SpawnLocation`)) (`KismetMathLibrary.Lerp` 0.0 -300.0 (/ (- (`KismetSystemLibrary.GetGameTimeInSeconds`) (`self.FallTime`)) (`self.RiseFallDuration`)))))
    (elif (> (`KismetSystemLibrary.GetGameTimeInSeconds`) (`self.RisenTime`))
      ;[1 1 1] Keep above ground
      (`self.K2_SetActorLocation` (`self.SpawnLocation`))
      (else
        ;[1 1 1] Rise the wall
        (`self.K2_SetActorLocation` (`KismetMathLibrary.MakeVector` (.x (`self.SpawnLocation`)) (.y (`self.SpawnLocation`)) (`KismetMathLibrary.Lerp` -300.0 0.0 (/ (- (`KismetSystemLibrary.GetGameTimeInSeconds`) (`self.SpawnTime`)) (`self.RiseFallDuration`)))))))))

(fn `UserConstructionScript`)